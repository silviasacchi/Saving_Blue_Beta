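; BP_EnemySpawn is a spawn point that creates escalating waves of BP_Swan enemies.
; On BeginPlay it binds SpawnEnemy to the respawn-enemies event in BP_EnemyGameMode.
; Each call spawns the current count of swans at the spawner's transform, adjusting for collisions but always spawning.
; It then raises the increment by one and adds it to the count, so wave size grows at an accelerating rate.
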(event `self.ReceiveBeginPlay`
  (bind _asbp_enemy_game_mode (cast `/Game/Blueprints/EnemyAI/BP_EnemyGameMode` (`GameplayStatics.GetGameMode`)))
  (add `/Game/Blueprints/EnemyAI/BP_EnemyGameMode.RespawnEnemies` _asbp_enemy_game_mode (delegate `SpawnEnemy`)))

(event `SpawnEnemy`
  (for _ (range (`self.EnemySwaned`))
    (`|SpawnActorFromClass` "/Game/Blueprints/Swans/BP_Swan.BP_Swan_C" (`self.GetTransform`) "AdjustIfPossibleButAlwaysSpawn" "OverrideRootScale" null null))
  (`/Engine/EditorBlueprintResources/StandardMacros.IncrementInt` (`self.EnemyIncrement`)
    (:`  `
      (set `self.EnemySwaned` (+ (`self.EnemySwaned`) (`self.EnemyIncrement`))))))

(fn `UserConstructionScript`)