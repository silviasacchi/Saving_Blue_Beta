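; BP_Swan is an enemy that homes in on the player character as soon as it spawns.
; On BeginPlay it increments BP_EnemyGameMode's EnemyAlive count and starts an AI MoveTo toward player 0.
; When it hits the player character it decrements that count, has the game mode check for remaining enemies, and destroys itself, without applying any damage.
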(event `self.ReceiveBeginPlay`
  (bind _asbp_enemy_game_mode (cast `/Game/Blueprints/EnemyAI/BP_EnemyGameMode` (`GameplayStatics.GetGameMode`)))
  (`/Engine/EditorBlueprintResources/StandardMacros.IncrementInt` (`/Game/Blueprints/EnemyAI/BP_EnemyGameMode.EnemyAlive` _asbp_enemy_game_mode)
    (:`  `
      (bind _asbp_third_person_character (cast `/Game/Blueprints/ThirdPerson/Blueprints/BP_ThirdPersonCharacter` (`GameplayStatics.GetPlayerCharacter` 0)))
      (`|AIMoveTo` self (0.0 0.0 0.0) _asbp_third_person_character))))

(event `self.ReceiveHit`
  (params (MyComp :type "PrimitiveComponent Object Reference") (Other :type "Actor Object Reference") (OtherComp :type "PrimitiveComponent Object Reference") (bSelfMoved :type Boolean) (HitLocation :type "Vector Structure") (HitNormal :type "Vector Structure") (NormalImpulse :type "Vector Structure") (Hit :type "HitResult Structure (by ref)"))
  (cast `/Game/Blueprints/ThirdPerson/Blueprints/BP_ThirdPersonCharacter` Other)
  (bind _asbp_enemy_game_mode (cast `/Game/Blueprints/EnemyAI/BP_EnemyGameMode` (`GameplayStatics.GetGameMode`)))
  (`/Engine/EditorBlueprintResources/StandardMacros.DecrementInt` (`/Game/Blueprints/EnemyAI/BP_EnemyGameMode.EnemyAlive` _asbp_enemy_game_mode)
    (:`  `
      (`/Game/Blueprints/EnemyAI/BP_EnemyGameMode.CheckEnemiesLeft` _asbp_enemy_game_mode)
      (`self.K2_DestroyActor`))))

(fn `UserConstructionScript`)